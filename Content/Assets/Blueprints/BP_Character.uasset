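; Player character that moves left and right along X, jumps and records picking up a BP_Collectible.
; Enhanced Input drives swept capsule offsets and flips the mesh to face travel, while jumping uses Character movement with boosted velocity and gravity.
; Damage, also self-inflicted with the M key, lowers Health and teleports the character to its start location.
; At zero Health the game pauses and shows the defeat widget with UI-only input.
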(event OnComponentBeginOverlap(CapsuleComponent)
  (params (OverlappedComponent :type Primitive%20Component%20Object%20Reference) (OtherActor :type Actor%20Object%20Reference) (OtherComp :type Primitive%20Component%20Object%20Reference) (OtherBodyIndex :type Integer) (bFromSweep :type Boolean) (SweepResult :type Hit%20Result%20Structure%20%28by%20ref%29))
  (Utilities|Casting|CastToBP_Collectible OtherActor)
  (Variables|Default|SetHasCollectible true))

(event Input|EnhancedActionEvents|EnhancedInputActionIA_Right
  (params (ActionValue :type Vector%202D%20Structure) (ElapsedSeconds :type Float%20%28double-precision%29) (TriggeredSeconds :type Float%20%28double-precision%29) (InputAction :type Input%20Action%20Object%20Reference :default "/Game/Assets/Input/IA_Right.IA_Right"))
  ;[1 1 1] Movement - Run and jump
  (:Triggered
    (Transformation|AddRelativeLocation (Variables|Collision|GetCapsuleComponent) (Math|Vector|MakeVector (* (Utilities|Time|GetWorldDeltaSeconds) (Variables|Default|GetSpeed)) 0.0 0.0) true false)
    (Transformation|SetRelativeRotation (Variables|Default|GetSM_Capsule) "0.000000,0.000000,0.000000" false false)))

(event Input|EnhancedActionEvents|EnhancedInputActionIA_Jump
  (params (ActionValue :type Boolean) (ElapsedSeconds :type Float%20%28double-precision%29) (TriggeredSeconds :type Float%20%28double-precision%29) (InputAction :type Input%20Action%20Object%20Reference :default "/Game/Assets/Input/IA_Jump.IA_Jump"))
  ;[1 1 1] Movement - Run and jump
  (:Triggered
    (Character|Jump))
  (:Completed
    (Character|StopJumping)))

(event Input|EnhancedActionEvents|EnhancedInputActionIA_Left
  (params (ActionValue :type Vector%202D%20Structure) (ElapsedSeconds :type Float%20%28double-precision%29) (TriggeredSeconds :type Float%20%28double-precision%29) (InputAction :type Input%20Action%20Object%20Reference :default "/Game/Assets/Input/IA_Left.IA_Left"))
  ;[1 1 1] Movement - Run and jump
  (:Triggered
    (Transformation|AddRelativeLocation (Variables|Collision|GetCapsuleComponent) (Math|Vector|MakeVector (* (Variables|Default|GetSpeed) (Utilities|Time|GetWorldDeltaSeconds) -1.0) 0.0 0.0) true false)
    (Transformation|SetRelativeRotation (Variables|Default|GetSM_Capsule) "0.000000,180.000000,0.000000" false false)))

(event EventBeginPlay
  (bind _returnvalue (Game|GetPlayerController 0))
  (bind _charactermovement (Variables|Character|GetCharacterMovement))
  ;[1 1 1] Input Mapping Setup
  (Variables|Default|SetPlayerStartLocation (Transformation|GetActorLocation))
  (Input|AddMappingContext (PlayerController|LocalPlayerSubsystems|GetEnhancedInputLocalPlayerSubsystem (Game|GetPlayerController (Game|GetPlayerState 0))) "/Game/Assets/Input/IMC_Character.IMC_Character" 0 "(bIgnoreAllPressedKeysUntilRelease=True,bForceImmediately=False)")
  ;[1 1 1] Movement - Run and jump
  (Variables|Default|SetJumpMaxHoldTime 0.0)
  (Variables|/Script/Engine.CharacterMovementComponent|SetJumpZVelocity _charactermovement (* (Variables|/Script/Engine.CharacterMovementComponent|GetJumpZVelocity _charactermovement) 1.5))
  (Variables|/Script/Engine.CharacterMovementComponent|SetGravityScale _charactermovement 2.0)
  (Variables|/Script/Engine.PlayerController|SetbShowMouseCursor _returnvalue false)
  (Input|SetInputModeGameOnly _returnvalue false))

(event Game|Damage|EventAnyDamage
  (params (Damage :type Float%20%28single-precision%29) (DamageType :type Damage%20Type%20Object%20Reference) (InstigatedBy :type Controller%20Object%20Reference) (DamageCauser :type Actor%20Object%20Reference))
  (bind _returnvalue (Game|GetPlayerController 0))
  (Variables|Default|SetHealth (- (Variables|Default|GetHealth) Damage))
  (if (<= (Variables|Default|GetHealth) 0.0)
    (Game|SetGamePaused true)
    (bind _returnvalue_2 (UserInterface|CreateWidget "/Game/Assets/Blueprints/WB_Defeat.WB_Defeat_C"))
    (UserInterface|Viewport|AddtoViewport _returnvalue_2 0)
    (Variables|/Script/Engine.PlayerController|SetbShowMouseCursor _returnvalue true)
    (Input|SetInputModeUIOnly _returnvalue _returnvalue_2 "DoNotLock" false)
    (else
      (Transformation|SetWorldLocation (Variables|Collision|GetCapsuleComponent) (Variables|Default|GetPlayerStartLocation) false true))))

(event EventTick
  (params (DeltaSeconds :type Float%20%28single-precision%29))
  (Variables|Default|SetDelta%20Seconds DeltaSeconds))

(event Input|KeyboardEvents|M
  (params (Key :type Key%20Structure :default "None"))
  (:Pressed
    (Game|Damage|ApplyDamage self 1.0 0 0)))

(fn ConstructionScript)